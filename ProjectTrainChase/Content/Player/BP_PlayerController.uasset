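; Player controller for BP_Player that handles movement input and the character's visual state on a plane.
; The Forward axis moves the pawn along its facing, while the Right axis turns it through yaw input.
; Each Tick swaps the plane's material for idle, forward or backward walking, and left or right turns.
; When PlayerHasFallen is set and the character is not airborne, a fallen-down material replaces these.
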(event `self.ReceiveBeginPlay`
  (bind _asbp_player (cast `/Game/Player/BP_Player` (`self.K2_GetPawn`)))
  (set `self.PlayerChar` _asbp_player))

(event `InputAxis|Forward`
  (params (AxisValue :type "Float (single-precision)"))
  (bind _returnvalue (`self.K2_GetPawn`))
  (`Pawn.AddMovementInput` _returnvalue (`self.GetActorForwardVector` _returnvalue) AxisValue false))

(event `InputAxis|Right`
  (params (AxisValue :type "Float (single-precision)"))
  (`self.AddYawInput` AxisValue))

(event `self.ReceiveTick`
  (params (DeltaSeconds :type "Float (single-precision)"))
  (bind _playerchar (`self.PlayerChar`))
  (bind _playersplane (`/Game/Player/BP_Player.PlayersPlane` _playerchar))
  ;[1 1 1] Switch between different materials when idle, moving forward, moving right and moving left
  (if (`self.PlayerHasFallen`)
    (if (`NavMovementComponent.IsFalling` (`Character.CharacterMovement` _playerchar))
      (if (and (== (`self.GetInputAxisValue`) 0.0) (== (`self.GetInputAxisValue`) 0.0)) :!label _label
        (`PrimitiveComponent.SetMaterial` _playersplane 0 "/Game/Assets/Player/M_IdleCenter.M_IdleCenter")
        (elif (and (!= (`self.GetInputAxisValue`) 0.0) (== (`self.GetInputAxisValue`) 0.0))
          (`PrimitiveComponent.SetMaterial` _playersplane 0 "/Game/Assets/Player/M_WalkCenter.M_WalkCenter")
          (elif (< (`self.GetInputAxisValue`) 0.0)
            (`PrimitiveComponent.SetMaterial` _playersplane 0 "/Game/Assets/Player/M_WalkLeft.M_WalkLeft")
            (else
              (`PrimitiveComponent.SetMaterial` _playersplane 0 "/Game/Assets/Player/M_WalkRight.M_WalkRight")))))
      (else
        (`PrimitiveComponent.SetMaterial` _playersplane 0 "/Game/Assets/Player/M_FallenDown.M_FallenDown")))
    (else
      (goto _label))))

(fn `UserConstructionScript`)