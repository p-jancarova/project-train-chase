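; Player character with a countdown that quits the game at zero, a coin balance display, a timed speed boost and a minimap.
; Tick prints the coins, adds consumed movement input as an unswept world offset, and uses Delay nodes as one-second clocks for the countdown and elapsed time.
; The SpeedUp input raises max walk speed, then SlowDown reverts it after a delay.
; BeginPlay adds the minimap widget.
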(event `self.ReceiveTick`
  (params (DeltaSeconds :type "Float (single-precision)"))
  (`KismetSystemLibrary.PrintString` (`KismetStringLibrary.Conv_IntToString` (`self.CollectedCoins`)) true true (struct :`R` 0.745098 :`G` 0.435294 :`B` 0.094118 :`A` 1.0) DeltaSeconds)
  (`KismetSystemLibrary.PrintString` "your bank balance:" true true (struct :`R` 0.746073 :`G` 0.436218 :`B` 0.096228 :`A` 1.0) DeltaSeconds)
  (`|ExecutionSequence`
    (:`then_0`
      (`KismetSystemLibrary.Delay` 1.0)
      (if (== (`self.Seconds`) 0)
        (if (== (`self.Minutes`) 0)
          (`KismetSystemLibrary.QuitGame` null "Quit")
          (else
            (set `self.Seconds` 59)
            (set `self.Minutes` (- (`self.Minutes`) 1))))
        (else
          (set `self.Seconds` (- (`self.Seconds`) 1)))))
    (:`then_1`
      (bind _returnvalue (`self.ConsumeMovementInputVector`))
      (`self.K2_AddActorWorldOffset` _returnvalue))
    (:`then_2`
      (`KismetSystemLibrary.Delay` 1.0)
      (if (== (`self.Current_seconds`) 59)
        (set `self.Current_seconds` 0)
        (set `self.Current_minutes` (+ (`self.Current_minutes`) 1))
        (else
          (set `self.Current_seconds` (+ (`self.Current_seconds`) 1)))))))

(event `InputAction|SpeedUp`
  (params (Key :type "Key Structure"))
  (:`Pressed`
    (`self.SpeedUp` 1000.0)
    (`KismetSystemLibrary.Delay` 5.0)
    (`self.SlowDown` 1000.0)))

(event `self.ReceiveBeginPlay`
  (bind _returnvalue (`|CreateWidget` "/Game/World/WB_minimap.WB_minimap_C" (`GameplayStatics.GetPlayerController` 0)))
  (`UserWidget.AddToViewport` _returnvalue 0))

(fn `SlowDown`
  (params (SpeedDecrement :type "Float (double-precision)"))
  (bind _charactermovement (`self.CharacterMovement`))
  (bind _output_get (set `CharacterMovementComponent.MaxWalkSpeed` (- (`CharacterMovementComponent.MaxWalkSpeed` _charactermovement) SpeedDecrement) _charactermovement))
  (`KismetSystemLibrary.PrintString` "SLOW DOWN")
  (`KismetSystemLibrary.PrintString` (`KismetStringLibrary.Conv_DoubleToString` _output_get)))

(fn `SpeedUp`
  (params (SpeedIncrement :type "Float (double-precision)"))
  (bind _charactermovement (`self.CharacterMovement`))
  (bind _output_get (set `CharacterMovementComponent.MaxWalkSpeed` (+ SpeedIncrement (`CharacterMovementComponent.MaxWalkSpeed` _charactermovement)) _charactermovement))
  (`KismetSystemLibrary.PrintString` "SPEED UP")
  (`KismetSystemLibrary.PrintString` (`KismetStringLibrary.Conv_DoubleToString` _output_get)))

(fn `UserConstructionScript`)