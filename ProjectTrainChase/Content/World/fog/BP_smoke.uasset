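; BP_smoke is a fog or smoke effect actor that switches on its Niagara effect at a set point on the game clock.
; It deactivates the Niagara component on BeginPlay.
; Every Tick it casts to BP_GameInstance, reads minutes and seconds, and activates the effect without a reset when they match the hard-coded time.
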(event `self.ReceiveBeginPlay`
  (`ActorComponent.Deactivate` (`self.Niagara`)))

(event `self.ReceiveTick`
  (params (DeltaSeconds :type "Float (single-precision)"))
  (bind _asbp_game_instance (cast `/Game/BP_GameInstance` (`GameplayStatics.GetGameInstance`)))
  (bind _minutes (`/Game/BP_GameInstance.GetMinutes` _asbp_game_instance))
  (bind _seconds (`/Game/BP_GameInstance.GetSeconds` _asbp_game_instance))
  (if (== _minutes 0)
    (if (== _seconds 15)
      (`ActorComponent.Activate` (`self.Niagara`) false))))

(fn `UserConstructionScript`)