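; BP_SmallRockObstacle is a small rock obstacle that trips the player on overlap.
; It launches BP_Player upward, flags PlayerHasFallen on BP_PlayerController and sets walk speed to zero.
; After a delay, it restores walk speed from BP_GameInstance's CharacterSpeed and clears the fallen flag.
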(event `self.ReceiveActorBeginOverlap`
  (params (OtherActor :type "Actor Object Reference"))
  (bind _asbp_player (cast `/Game/Player/BP_Player` OtherActor))
  (`Character.LaunchCharacter` _asbp_player (0.0 0.0 500.0) false false)
  (bind _asbp_player_controller (cast `/Game/Player/BP_PlayerController` (`GameplayStatics.GetPlayerController` 0)))
  (set `/Game/Player/BP_PlayerController.PlayerHasFallen` true _asbp_player_controller)
  (bind _charactermovement (`Character.CharacterMovement` _asbp_player))
  (set `CharacterMovementComponent.MaxWalkSpeed` 0.0 _charactermovement)
  (`KismetSystemLibrary.Delay` 4.0)
  (bind _asbp_game_instance (cast `/Game/BP_GameInstance` (`GameplayStatics.GetGameInstance`)))
  (set `CharacterMovementComponent.MaxWalkSpeed` (`/Game/BP_GameInstance.CharacterSpeed` _asbp_game_instance) _charactermovement)
  (set `/Game/Player/BP_PlayerController.PlayerHasFallen` false _asbp_player_controller)
  (`KismetSystemLibrary.Delay` 1.0))

(fn `UserConstructionScript`)