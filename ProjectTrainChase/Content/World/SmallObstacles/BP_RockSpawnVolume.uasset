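; BP_RockSpawnVolume is a box volume that scatters small rock obstacles inside itself when play begins.
; On BeginPlay it picks a random count between MinNumOfRocks and MaxNumOfRocks and spawns that many BP_SmallRockObstacle actors.
; Each location is a random per-axis offset from the box's scaled extent added to its world location, so box rotation is ignored.
; Rocks spawn with zero rotation and unit scale.
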(event `self.ReceiveBeginPlay`
  (bind _boxcollision (`self.BoxCollision`))
  (bind _x (.x (`BoxComponent.GetScaledBoxExtent` _boxcollision)))
  (bind _y (.y (`BoxComponent.GetScaledBoxExtent` _boxcollision)))
  (bind _z (.z (`BoxComponent.GetScaledBoxExtent` _boxcollision)))
  (for _ (range 1 (+ (`KismetMathLibrary.RandomIntegerInRange` (`self.MinNumOfRocks`) (`self.MaxNumOfRocks`)) 1))
    (bind _result (`/Engine/EditorBlueprintResources/StandardMacros.NegateFloat` _x)
      (:`  `
        (bind _result_2 (`/Engine/EditorBlueprintResources/StandardMacros.NegateFloat` _y)
          (:`  `
            (bind _result_3 (`/Engine/EditorBlueprintResources/StandardMacros.NegateFloat` _z)
              (:`  `
                (`|SpawnActorFromClass` "/Game/World/SmallObstacles/BP_SmallRockObstacle.BP_SmallRockObstacle_C" (`KismetMathLibrary.MakeTransform` (+ (`KismetMathLibrary.MakeVector` (`KismetMathLibrary.RandomFloatInRange` _result _x) (`KismetMathLibrary.RandomFloatInRange` _result_2 _y) (`KismetMathLibrary.RandomFloatInRange` _result_3 _z)) (`SceneComponent.K2_GetComponentLocation` _boxcollision))) "Undefined" "OverrideRootScale" null null)))))))))

(fn `UserConstructionScript`)