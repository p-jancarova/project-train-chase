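; BP_Crowd is a crowd zone actor that slows the player while they overlap it.
; On begin overlap it casts to BP_Player and sets the CharacterMovement max walk speed to a low fixed value.
; On end overlap it restores the walk speed from CharacterSpeed in BP_GameInstance.
; Both events print a debug message, and no other logic runs.
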(event `self.ReceiveActorBeginOverlap`
  (params (OtherActor :type "Actor Object Reference"))
  (bind _asbp_player (cast `/Game/Player/BP_Player` OtherActor))
  (set `CharacterMovementComponent.MaxWalkSpeed` 50.0 (`Character.CharacterMovement` _asbp_player))
  (`KismetSystemLibrary.PrintString` "SPEED REDUCED - CROWD"))

(event `self.ReceiveActorEndOverlap`
  (params (OtherActor :type "Actor Object Reference"))
  (bind _asbp_player (cast `/Game/Player/BP_Player` OtherActor))
  (bind _asbp_game_instance (cast `/Game/BP_GameInstance` (`GameplayStatics.GetGameInstance`)))
  (set `CharacterMovementComponent.MaxWalkSpeed` (`/Game/BP_GameInstance.CharacterSpeed` _asbp_game_instance) (`Character.CharacterMovement` _asbp_player))
  (`KismetSystemLibrary.PrintString` "Speed recovered!"))

(fn `UserConstructionScript`)