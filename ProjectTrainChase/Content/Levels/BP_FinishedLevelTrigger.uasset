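; BP_FinishedLevelTrigger is an end-of-level trigger that checks whether the player has a ticket when they overlap it.
; Players with a ticket go straight to the L_LevelStats level.
; Without one, it deducts the penalty price from the coins stored in BP_GameInstance and flags the penalty as paid before opening that level.
; If coins fall short, it shows the GameOver widget, enables the mouse cursor and pauses the game.
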(event `self.ReceiveActorBeginOverlap`
  (params (OtherActor :type "Actor Object Reference"))
  (bind _asbp_player (cast `/Game/Player/BP_Player` OtherActor))
  (if (`/Game/Player/BP_Player.HasTicket` _asbp_player)
    (`GameplayStatics.OpenLevelBySoftObjectPtr` "/Game/Levels/L_LevelStats.L_LevelStats" :!label _label)
    (else
      (bind _asbp_game_instance (cast `/Game/BP_GameInstance` (`GameplayStatics.GetGameInstance`)))
      (bind _penaltyprice (`/Game/BP_GameInstance.PenaltyPrice` _asbp_game_instance))
      (bind _collectedcoins (`/Game/BP_GameInstance.CollectedCoins` _asbp_game_instance))
      (if (<= _penaltyprice _collectedcoins)
        (set `/Game/BP_GameInstance.CollectedCoins` (- _collectedcoins _penaltyprice) _asbp_game_instance)
        (set `/Game/BP_GameInstance.PaidPenalty` true _asbp_game_instance)
        (goto _label)
        (else
          (bind _returnvalue (`|CreateWidget` "/Game/Player/GameOver.GameOver_C"))
          (`UserWidget.AddToViewport` _returnvalue 0)
          (set `PlayerController.bShowMouseCursor` true (`GameplayStatics.GetPlayerController` 0))
          (`GameplayStatics.SetGamePaused` true))))))

(fn `UserConstructionScript`)