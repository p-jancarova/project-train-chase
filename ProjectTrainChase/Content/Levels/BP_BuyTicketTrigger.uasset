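; Trigger actor that sells the player a ticket when overlapped, paid for with collected coins.
; Any overlap checks player pawn 0 rather than the overlapping actor, reading HasTicket on BP_Player.
; With enough coins in BP_GameInstance, it deducts TicketPrice, sets HasTicket and plays a cash register sound.
; Otherwise, it briefly shows an already-owned or not-enough-money widget, removed after a short delay.
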(event `self.ReceiveActorBeginOverlap`
  (params (OtherActor :type "Actor Object Reference"))
  (bind _asbp_player (cast `/Game/Player/BP_Player` (`GameplayStatics.GetPlayerPawn` 0)))
  (if (`/Game/Player/BP_Player.HasTicket` _asbp_player)
    (bind _returnvalue (`|CreateWidget` "/Game/Levels/UI_CarefulMessage.UI_CarefulMessage_C"))
    (set `/Game/Levels/UI_CarefulMessage.MessageString` "You already have a ticket!" _returnvalue)
    (`UserWidget.AddToViewport` _returnvalue 0)
    (`KismetSystemLibrary.Delay` 1.0)
    (`Widget.RemoveFromParent` _returnvalue)
    (else
      (bind _asbp_game_instance (cast `/Game/BP_GameInstance` (`GameplayStatics.GetGameInstance`)))
      (bind _collectedcoins (`/Game/BP_GameInstance.CollectedCoins` _asbp_game_instance))
      (bind _ticketprice (`/Game/BP_GameInstance.TicketPrice` _asbp_game_instance))
      (if (>= _collectedcoins _ticketprice)
        (set `/Game/BP_GameInstance.CollectedCoins` (- _collectedcoins _ticketprice) _asbp_game_instance)
        (set `/Game/Player/BP_Player.HasTicket` true _asbp_player)
        (`GameplayStatics.PlaySoundAtLocation` "/Game/audio/cash-register-purchase-87313.cash-register-purchase-87313" (`self.K2_GetActorLocation`) (struct) 1.0 1.0 0.0 null null null)
        (else
          (bind _returnvalue_2 (`|CreateWidget` "/Game/Levels/UI_NotEnoughMoneyMessage.UI_NotEnoughMoneyMessage_C"))
          (`UserWidget.AddToViewport` _returnvalue_2 0)
          (`KismetSystemLibrary.Delay` 1.0)
          (`Widget.RemoveFromParent` _returnvalue_2))))))

(fn `UserConstructionScript`)