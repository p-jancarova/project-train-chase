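; BP_BounceTrigger is a trigger actor that knocks the player away and flashes a warning.
; On overlap with BP_Player, it launches the character along the normalized direction from the trigger to the player, adding a fixed-strength impulse to the current velocity.
; It also shows a UI_WarningMessage widget for one second, using the stored CarefulMessage reference to avoid duplicates while one is visible.
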(event `self.ReceiveActorBeginOverlap`
  (params (OtherActor :type "Actor Object Reference"))
  (bind _asbp_player (cast `/Game/Player/BP_Player` OtherActor))
  (`Character.LaunchCharacter` _asbp_player (* (`KismetMathLibrary.Normal` (- (`self.K2_GetActorLocation` _asbp_player) (`self.K2_GetActorLocation`))) 1000.0) false false)
  (if (not (`KismetSystemLibrary.IsValid` (`self.CarefulMessage`)))
    (bind _returnvalue (`|CreateWidget` "/Game/Levels/WidgetsAndUI/UI_WarningMessage.UI_WarningMessage_C"))
    (bind _output_get (set `self.CarefulMessage` _returnvalue))
    (`UserWidget.AddToViewport` _output_get 0)
    (`KismetSystemLibrary.Delay` 1.0)
    (`Widget.RemoveFromParent` _output_get)
    (set `self.CarefulMessage` null)))

(fn `UserConstructionScript`)