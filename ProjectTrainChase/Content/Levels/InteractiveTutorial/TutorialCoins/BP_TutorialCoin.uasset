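; Tutorial coin that spins and guides collection through a fixed sequence of positions in the interactive tutorial level.
; A box overlap waits briefly, then adds a coin to both the game instance and player count.
; A sequence counter moves the same actor to each hard-coded spot with a sound, rather than spawning new coins.
; The final pickup fires CoinsFinished and destroys the coin.
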(event `self.ReceiveBeginPlay`)

(event `self.ReceiveTick`
  (params (DeltaSeconds :type "Float (single-precision)"))
  (bind _cylinder (`self.Cylinder`))
  (bind (_relativerotation_roll _relativerotation_pitch _relativerotation_yaw) (`KismetMathLibrary.BreakRotator` (`SceneComponent.RelativeRotation` _cylinder)))
  (`SceneComponent.K2_SetRelativeRotation` _cylinder (`KismetMathLibrary.MakeRotator` (+ _relativerotation_roll 2.0) _relativerotation_pitch _relativerotation_yaw) false false))

(event `self.Box.OnComponentBeginOverlap`
  (params (OverlappedComponent :type "PrimitiveComponent Object Reference") (OtherActor :type "Actor Object Reference") (OtherComp :type "PrimitiveComponent Object Reference") (OtherBodyIndex :type Integer) (bFromSweep :type Boolean) (SweepResult :type "HitResult Structure (by ref)"))
  (bind _sequencenumber (`self.SequenceNumber`))
  (bind _asbp_player (cast `/Game/Player/BP_Player` (`GameplayStatics.GetPlayerCharacter` 0)))
  (`KismetSystemLibrary.Delay` 0.2)
  (bind _asbp_game_instance (cast `/Game/BP_GameInstance` (`GameplayStatics.GetGameInstance`)))
  (`/Game/BP_GameInstance.AddCoin` _asbp_game_instance)
  (set `/Game/Player/BP_Player.CollectedCoins` (+ (`/Game/Player/BP_Player.CollectedCoins` _asbp_player) 1) _asbp_player)
  (if (== _sequencenumber 0)
    (`self.K2_SetActorLocation` (800.0 800.0 60.0))
    (`GameplayStatics.PlaySoundAtLocation` "/Game/AudioFiles/CoinSound/coinSound.coinSound" (800.0 800.0 60.0) (struct) 1.0 1.0 0.0 null null null)
    (set `self.SequenceNumber` (+ _sequencenumber 1))
    (elif (== _sequencenumber 1)
      (`self.K2_SetActorLocation` (800.0 -800.0 60.0))
      (`GameplayStatics.PlaySoundAtLocation` "/Game/AudioFiles/CoinSound/coinSound.coinSound" (800.0 -800.0 60.0) (struct) 1.0 1.0 0.0 null null null)
      (set `self.SequenceNumber` (+ _sequencenumber 1))
      (elif (== _sequencenumber 2)
        (`self.K2_SetActorLocation` (0.0 800.0 60.0))
        (`GameplayStatics.PlaySoundAtLocation` "/Game/AudioFiles/CoinSound/coinSound.coinSound" (1600.0 800.0 60.0) (struct) 1.0 1.0 0.0 null null null)
        (set `self.SequenceNumber` (+ _sequencenumber 1))
        (elif (== _sequencenumber 3)
          (`self.K2_SetActorLocation` (0.0 -800.0 60.0))
          (`GameplayStatics.PlaySoundAtLocation` "/Game/AudioFiles/CoinSound/coinSound.coinSound" (1600.0 -800.0 60.0) (struct) 1.0 1.0 0.0 null null null)
          (set `self.SequenceNumber` (+ _sequencenumber 1))
          (else
            (`self.CoinsFinished`)
            (`self.K2_DestroyActor`)))))))

(fn `UserConstructionScript`)