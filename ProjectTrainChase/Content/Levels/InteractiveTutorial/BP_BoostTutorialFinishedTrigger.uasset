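; One-shot trigger in the interactive tutorial that marks the end of the boost section and introduces the obstacles section.
; On any actor overlap, it creates a UI_TutorialMessage widget with the obstacles title and instructions, pauses the game and shows the mouse cursor with input mode set to game only.
; It then fires the BoostFinished dispatcher and destroys itself.
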(event `self.ReceiveActorBeginOverlap`
  (params (OtherActor :type "Actor Object Reference"))
  (bind _returnvalue (`GameplayStatics.GetPlayerController` 0))
  (`WidgetBlueprintLibrary.SetInputMode_GameOnly` _returnvalue)
  (bind _returnvalue_2 (`|CreateWidget` "/Game/Levels/InteractiveTutorial/UI_TutorialMessage.UI_TutorialMessage_C"))
  (set `/Game/Levels/InteractiveTutorial/UI_TutorialMessage.TutorialTitleString` (`self.ObstaclesTutorialTitle`) _returnvalue_2)
  (set `/Game/Levels/InteractiveTutorial/UI_TutorialMessage.TutorialInstructionsString` (`self.ObstaclesTutorialInstructions`) _returnvalue_2)
  (`UserWidget.AddToViewport` _returnvalue_2 0)
  (`GameplayStatics.SetGamePaused` true)
  (set `PlayerController.bShowMouseCursor` true _returnvalue)
  (`self.BoostFinished`)
  (`self.K2_DestroyActor`))

(fn `UserConstructionScript`)