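; Overlap trigger that ends the tutorial at the finish of the obstacles segment in the interactive tutorial level.
; On any actor overlap it switches input to UI only, then disables the player character's movement if it is a BP_Player.
; It then shows a UI_TutorialMessage with the end-of-tutorial text and the mouse cursor, signals the end of the tutorial and destroys itself.
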(event `self.ReceiveActorBeginOverlap`
  (params (OtherActor :type "Actor Object Reference"))
  (bind _returnvalue (`GameplayStatics.GetPlayerController` 0))
  (`WidgetBlueprintLibrary.SetInputMode_UIOnlyEx` _returnvalue null)
  (bind _asbp_player (cast `/Game/Player/BP_Player` (`GameplayStatics.GetPlayerCharacter` 0)))
  (`CharacterMovementComponent.DisableMovement` (`Character.CharacterMovement` _asbp_player))
  (bind _returnvalue_2 (`|CreateWidget` "/Game/Levels/InteractiveTutorial/UI_TutorialMessage.UI_TutorialMessage_C"))
  (set `/Game/Levels/InteractiveTutorial/UI_TutorialMessage.TutorialTitleString` (`self.EndTutorialTitle`) _returnvalue_2)
  (set `/Game/Levels/InteractiveTutorial/UI_TutorialMessage.TutorialInstructionsString` (`self.EndTutorialInstructions`) _returnvalue_2)
  (`UserWidget.AddToViewport` _returnvalue_2 0)
  (set `PlayerController.bShowMouseCursor` true _returnvalue)
  (`self.EndOfTutorial`)
  (`self.K2_DestroyActor`))

(fn `UserConstructionScript`)